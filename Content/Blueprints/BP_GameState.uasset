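; Game state that runs a timed survival round, tracking time played, difficulty and end-of-game status.
; A looping one-second timer awards each player score by difficulty and periodically spawns a randomly placed BP_Boulder while raising difficulty.
; Ending stops the timer, updates HP and highest score in BP_GameInstance, and shows the HUD restart prompt.
; Restarting reloads the level, resetting HP and highest score when HP is zero.
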(event `self.ReceiveBeginPlay`
  (`self.StartGameEvent`))

(event `StartGameEvent`
  (bind _returnvalue (`KismetSystemLibrary.K2_SetTimerDelegate` (delegate `MainTimerEvent`) 1.0 true))
  (set `self.Timer` _returnvalue)
  (set `self.IsGameEnded` false)
  (bind _asbp_hud (cast `/Game/Blueprints/BP_HUD` (`PlayerController.GetHUD` (`GameplayStatics.GetPlayerController` 0))))
  (`/Game/Blueprints/BP_HUD.ShowRestartGameEvent` _asbp_hud false))

(event `MainTimerEvent`
  (`/Engine/EditorBlueprintResources/StandardMacros.IncrementInt` (`self.TimePlayed`)
    (:`  `
      (for _array_element (`self.PlayerArray`)
        (bind _asbp_player_state (cast `/Game/Blueprints/BP_PlayerState` _array_element))
        (`/Game/Blueprints/BP_PlayerState.AddPlayerScore` _asbp_player_state (`self.Difficulty`)))
      (if (== (mod (`self.TimePlayed`) 5) 0)
        (`|SpawnActorFromClass` "/Game/Blueprints/BP_Boulder.BP_Boulder_C" (`KismetMathLibrary.MakeTransform` (`KismetMathLibrary.MakeVector` (`KismetMathLibrary.RandomFloatInRange` 110.0 2890.0) (`KismetMathLibrary.RandomFloatInRange` 110.0 1580.0) 100.0) (`KismetMathLibrary.MakeRotator` 0.0 0.0 (`KismetMathLibrary.RandomFloatInRange` 0.0 360.0))) "AdjustIfPossibleButAlwaysSpawn" "MultiplyWithRoot" null null)
        (`self.IncreaseDifficulty`)))))

(event `EndGameEvent`
  (`|ExecutionSequence`
    (:`then_0`
      (bind _asbp_game_instance (cast `/Game/Blueprints/BP_GameInstance` (`GameplayStatics.GetGameInstance`)))
      (`/Game/Blueprints/BP_GameInstance.ChangeHPScore` _asbp_game_instance)
      (`/Game/Blueprints/BP_GameInstance.UpdateCurrentHP` _asbp_game_instance (`/Game/Blueprints/BP_GameInstance.GetCurrentHP` _asbp_game_instance))
      (bind _asbp_hud (cast `/Game/Blueprints/BP_HUD` (`PlayerController.GetHUD` (`GameplayStatics.GetPlayerController` 0))))
      (`/Game/Blueprints/BP_HUD.ShowRestartGameEvent` _asbp_hud true))
    (:`then_1`
      (`KismetSystemLibrary.K2_ClearAndInvalidateTimerHandle` (`self.Timer`))
      (set `self.IsGameEnded` true)
      (bind _asbp_game_instance_2 (cast `/Game/Blueprints/BP_GameInstance` (`GameplayStatics.GetGameInstance`)))
      (for _array_element (`self.PlayerArray`)
        (bind _asbp_player_state (cast `/Game/Blueprints/BP_PlayerState` _array_element))
        (`/Game/Blueprints/BP_GameInstance.UpdateHighestScore` _asbp_game_instance_2 (`/Game/Blueprints/BP_PlayerState.GetPlayerScore` _asbp_player_state))))))

(event `RestartGameEvent`
  (bind _asbp_hud (cast `/Game/Blueprints/BP_HUD` (`PlayerController.GetHUD` (`GameplayStatics.GetPlayerController` 0))))
  (`/Game/Blueprints/BP_HUD.ShowRestartGameEvent` _asbp_hud false)
  (bind _returnvalue (`GameplayStatics.GetCurrentLevelName` true))
  (`GameplayStatics.OpenLevel` (`KismetStringLibrary.Conv_StringToName` _returnvalue))
  (bind _asbp_game_instance (cast `/Game/Blueprints/BP_GameInstance` (`GameplayStatics.GetGameInstance`)))
  (if (== (`/Game/Blueprints/BP_GameInstance.GetCurrentHP` _asbp_game_instance) 0)
    (set `/Game/Blueprints/BP_GameInstance.CurrentHP` 3 _asbp_game_instance)
    (set `/Game/Blueprints/BP_GameInstance.HighestScore` 0 _asbp_game_instance)))

(fn `GetDifficulty`
  (returns (Difficulty :type Integer))
  (return (`self.Difficulty`)))

(fn `GetIsGameEnded`
  (returns (IsGameEnded :type Boolean))
  (return (`self.IsGameEnded`)))

(fn `GetTimePlayed`
  (returns (TimePlayed :type Integer))
  (return (`self.TimePlayed`)))

(fn `IncreaseDifficulty`
  (`/Engine/EditorBlueprintResources/StandardMacros.IncrementInt` (`self.Difficulty`)))

(fn `UserConstructionScript`)