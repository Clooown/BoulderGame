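; BP_Boulder is a moving hazard that kills the player on contact and ends the game.
; Each tick it sweeps forward at its Speed, and on hitting anything other than the player it bounces by mirroring its forward vector on the hit normal.
; Hitting the player destroys both actors with explosion effects and calls EndGameEvent on BP_GameState.
; TurnToTarget aims it horizontally at a given actor.
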(event `self.ReceiveHit`
  (params (MyComp :type "PrimitiveComponent Object Reference") (Other :type "Actor Object Reference") (OtherComp :type "PrimitiveComponent Object Reference") (bSelfMoved :type Boolean) (HitLocation :type "Vector Structure") (HitNormal :type "Vector Structure") (NormalImpulse :type "Vector Structure") (Hit :type "HitResult Structure (by ref)"))
  (bind _returnvalue_location (`KismetMathLibrary.BreakTransform` (`self.GetTransform`)))
  (bind _asbp_player_character (cast `/Game/Blueprints/BP_PlayerCharacter` Other)
    (:`then`
      (`self.K2_DestroyActor` _asbp_player_character)
      (`GameplayStatics.SpawnEmitterAtLocation` "/Game/StarterContent/Particles/P_Explosion.P_Explosion" _returnvalue_location)
      (`GameplayStatics.PlaySoundAtLocation` "/Game/StarterContent/Audio/Explosion_Cue.Explosion_Cue" _returnvalue_location (struct) 1.0 1.0 0.0 null null null null)
      (`self.K2_DestroyActor`)
      (bind _asbp_game_state (cast `/Game/Blueprints/BP_GameState` (`GameplayStatics.GetGameState`)))
      (`/Game/Blueprints/BP_GameState.EndGameEvent` _asbp_game_state))
    (:`CastFailed`
      (`self.K2_SetActorRotation` (`KismetMathLibrary.MakeRotFromX` (`KismetMathLibrary.MirrorVectorByNormal` (`self.GetActorForwardVector`) HitNormal))))))

(event `self.ReceiveTick`
  (params (DeltaSeconds :type "Float (single-precision)"))
  (`self.K2_AddActorWorldOffset` (* (* DeltaSeconds (`self.Speed`)) (`self.GetActorForwardVector`)) true))

(fn `UserConstructionScript`)